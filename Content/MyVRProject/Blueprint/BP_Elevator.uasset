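; BP_Elevator is a VR elevator actor that moves between floor positions when its VR button changes state.
; The first trip uses a timeline to lerp from the BeginPlay location to Location1F, then clears IsFirst.
; Later presses alternate through a FlipFlop, playing or reversing a second timeline between Location1F and Location2F.
; Each press disables the button for a fixed delay, then re-enables and resets it without retriggering its event.
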(event OnButtonStateChanged(VRButton)
  (params (ButtonState :type Boolean) (InteractingActor :type Actor%20Object%20Reference) (InteractingComponent :type Primitive%20Component%20Object%20Reference))
  (bind _vrbutton (Variables|Default|GetVRButton))
  ;[1 1 1] 按钮设置
  (Variables|/Script/VRExpansionPlugin.VRButtonComponent|SetbIsEnabled (Variables|Default|GetVRButton) false)
  (CallFunction|ElevatorUpDown)
  (Utilities|FlowControl|Delay 5.0)
  (Variables|/Script/VRExpansionPlugin.VRButtonComponent|SetbIsEnabled _vrbutton true)
  (Class|VRButtonComponent|SetButtonState _vrbutton false false false)
  (Default|SetColor _vrbutton))

(event Custom|ElevatorUpDown
  (if (Variables|Default|GetIs%20First)
    (bind _alpha (Timeline|时间轴 Play)
      (:Update
        (Transformation|SetActorLocation (Math|Vector|Lerp(Vector) (Variables|Default|GetInitialLocation) (Variables|Default|GetLocation_1F) _alpha) false false))
      (:Finished
        (Variables|Default|SetIs%20First false)))
    (else
      (Utilities|FlowControl|FlipFlop
        (:A
          (bind _alpha_2 (Timeline|时间轴_0 Play)
            (:Update
              (Transformation|SetActorLocation (Math|Vector|Lerp(Vector) (Variables|Default|GetLocation_1F) (Variables|Default|GetLocation_2F) _alpha_2) false false))))
        (:B
          (Timeline|时间轴_0 Reverse))))))

(event EventBeginPlay
  (Variables|Default|SetInitialLocation (Transformation|GetActorLocation)))

(event Collision|EventActorBeginOverlap
  (params (OtherActor :type Actor%20Object%20Reference)))

(event EventTick
  (params (DeltaSeconds :type Float%20%28single-precision%29)))

(fn ConstructionScript)