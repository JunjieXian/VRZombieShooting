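; VR player character with thumbstick movement, two-handed grabbing, held-object use, a left-hand menu and HP/ammo UI.
; Grips pick the highest-priority VRGripInterface object from a sphere trace, routing grab and drop through server or client RPCs by replication type.
; Slot grips attach hand meshes through proxies with hand-socket pose snapshots.
; Gripping at the props box spawns magazines from reserve ammo; OnRep CurrentHP drives death fade and destruction.
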(event OnGripOutOfRange(RightMotionController)
  (params (GripInformation :type BP%20Actor%20Grip%20Information%20Structure%20%28by%20ref%29) (Distance :type Float%20%28single-precision%29))
  ;[0 1 0.1887] Grip
  ;;[1 1 1] 被抓取物体因被阻挡导致超出距离后丢弃抓取物
  (if (>= Distance 1e+02)
    (Grip|DropAllGripObjects (Variables|Default|GetRightMotionController) (Variables|Default|GetLeftMotionController))))

(event OnGripOutOfRange(LeftMotionController)
  (params (GripInformation :type BP%20Actor%20Grip%20Information%20Structure%20%28by%20ref%29) (Distance :type Float%20%28single-precision%29))
  ;[0 1 0.1887] Grip
  ;;[1 1 1] 被抓取物体因被阻挡导致超出距离后丢弃抓取物
  (if (>= Distance 1e+02)
    (Grip|DropAllGripObjects (Variables|Default|GetLeftMotionController) (Variables|Default|GetRightMotionController))))

(event Custom|TryToGrab_Server
  (params (CallingMotionController :type Grip%20Motion%20Controller%20Component%20Object%20Reference) (OtherMotionController :type Grip%20Motion%20Controller%20Component%20Object%20Reference) (ObjectToGrip :type Object%20Object%20Reference) (ObjectTransform :type Transform) (isSlotRelativeGrip :type Boolean) (SlotName :type Name) (BoneName :type Name) (isSecondaryGrip :type Boolean))
  ;[0 1 0.1887] Grip
  ;;[0.9326 1 0] Grip&Drop RPCs
  (Grip|GrabObject CallingMotionController OtherMotionController ObjectToGrip ObjectTransform isSlotRelativeGrip SlotName BoneName isSecondaryGrip))

(event Custom|TryToGrab_Client
  (params (CallingMotionController :type Grip%20Motion%20Controller%20Component%20Object%20Reference) (OtherMotionController :type Grip%20Motion%20Controller%20Component%20Object%20Reference) (ObjectToGrip :type Object%20Object%20Reference) (ObjectTransform :type Transform%20%28by%20ref%29) (isSlotRelativeGrip :type Boolean) (SlotName :type Name) (BoneName :type Name) (isSecondaryGrip :type Boolean))
  ;[0 1 0.1887] Grip
  ;;[0.9326 1 0] Grip&Drop RPCs
  (Grip|GrabObject CallingMotionController OtherMotionController ObjectToGrip ObjectTransform isSlotRelativeGrip SlotName BoneName isSecondaryGrip))

(event Custom|UpdateBulletNumWidget
  (params (CurrentBullets :type Integer))
  ;[1 0.3166 0.7445] UI更新
  (bind _vrplayercontroller (Variables|Default|GetVRPlayerController)
    (:then
      (Default|UpdateBulltesNumUI _vrplayercontroller CurrentBullets (Variables|Gun|GetTotalBullets)))
    (:else)))

(event Custom|UpdateHPWidget
  (params (CurrentHP :type Float%20%28double-precision%29))
  ;[1 0.3166 0.7445] UI更新
  (bind _vrplayercontroller (Variables|Default|GetVRPlayerController)
    (:then
      (Default|UpdateHPPercentUI _vrplayercontroller CurrentHP (.maxhp (Variables|Default|GetCharcAttribute))))
    (:else)))

(event Custom|TryToDrop_Server
  (params (MotionController :type Grip%20Motion%20Controller%20Component%20Object%20Reference) (ObjectToDrop :type Object%20Object%20Reference) (GripIDToDrop :type Byte) (isSecondary :type Boolean))
  ;[0 1 0.1887] Grip
  ;;[0.9326 1 0] Grip&Drop RPCs
  (Grip|DropObject MotionController ObjectToDrop GripIDToDrop isSecondary))

(event Custom|TryToDrop_Client
  (params (MotionController :type Grip%20Motion%20Controller%20Component%20Object%20Reference) (ObjectToDrop :type Object%20Object%20Reference) (GripIDToDrop :type Byte) (isSecondary :type Boolean))
  ;[0 1 0.1887] Grip
  ;;[0.9326 1 0] Grip&Drop RPCs
  (Grip|DropObject MotionController ObjectToDrop GripIDToDrop isSecondary))

(event Input|EnhancedActionEvents|EnhancedInputActionUseHeldObjectRight
  (params (ActionValue :type Boolean) (ElapsedSeconds :type Float%20%28double-precision%29) (TriggeredSeconds :type Float%20%28double-precision%29) (InputAction :type Input%20Action%20Object%20Reference :default "/Game/VRE/Input/Actions/UseHeldObjectRight.UseHeldObjectRight"))
  (bind _rightmotioncontroller (Variables|Default|GetRightMotionController))
  (bind _rwidgetinteraction (Variables|Default|GetRWidgetInteraction))
  (bind _leftmotioncontroller (Variables|Default|GetLeftMotionController))
  ;[1 0.4104 0] Trigger Used
  (:Started
    (bind _wasovered (TriggerUse|IsOverWidgetUse _rwidgetinteraction true))
    (if (not _wasovered)
      (TriggerUse|UseHeldObject _rightmotioncontroller _leftmotioncontroller true)))
  (:Completed
    (bind _wasovered_2 (TriggerUse|IsOverWidgetUse _rwidgetinteraction false))
    (if (not _wasovered_2)
      (TriggerUse|UseHeldObject _rightmotioncontroller _leftmotioncontroller false))))

(event Input|EnhancedActionEvents|EnhancedInputActionAlternateGripLeft
  (params (ActionValue :type Boolean) (ElapsedSeconds :type Float%20%28double-precision%29) (TriggeredSeconds :type Float%20%28double-precision%29) (InputAction :type Input%20Action%20Object%20Reference :default "/Game/VRE/Input/Actions/AlternateGripLeft.AlternateGripLeft"))
  ;[1 1 1] 左手柄X/A键换出菜单，位于左手上方
  (:Started
    (Utilities|FlowControl|FlipFlop
      (:A
        (bind _returnvalue (Game|SpawnActorfromClass "/Game/MyVRProject/Blueprint/UI/BP_UIPlayerMenu.BP_UIPlayerMenu_C" (Transformation|GetWorldTransform (Variables|Default|GetLeftMotionController)) "Undefined" 0 (Game|GetInstigator)))
        (bind _output_get (Variables|Default|SetUIMenu _returnvalue))
        (Transformation|AttachComponentToComponent _output_get (Variables|Default|GetLeftMotionController) "None" "KeepRelative" "KeepRelative" "KeepWorld" true)
        (Transformation|SetActorRelativeTransform _output_get (Math|Transform|MakeTransform "18.000000,0.000000,20.000000" "40.000000,180.000000,0.000000" "0.200000,0.200000,0.200000") false false))
      (:B
        (bind _uimenu (Variables|Default|GetUIMenu)
          (:then
            (Actor|DestroyActor _uimenu))
          (:else))))))

(event Input|EnhancedActionEvents|EnhancedInputActionMotionControllerThumbLeft_X
  (params (ActionValue :type Float%20%28double-precision%29) (ElapsedSeconds :type Float%20%28double-precision%29) (TriggeredSeconds :type Float%20%28double-precision%29) (InputAction :type Input%20Action%20Object%20Reference :default "/Game/VRE/Input/Actions/MotionControllerThumbLeft_X.MotionControllerThumbLeft_X"))
  (bind _vrreplicatedcamera (Variables|Default|GetVRReplicatedCamera))
  (bind _returnvalue (Math|Vector|GetRightVector _vrreplicatedcamera))
  ;[1 1 1] Movement
  (:Triggered
    (Pawn|Input|AddMovementInput (Math|Vector|MakeVector (.x _returnvalue) (.y _returnvalue) 0.0) ActionValue false)))

(event Input|EnhancedActionEvents|EnhancedInputActionPrimaryGripLeft
  (params (ActionValue :type Boolean) (ElapsedSeconds :type Float%20%28double-precision%29) (TriggeredSeconds :type Float%20%28double-precision%29) (InputAction :type Input%20Action%20Object%20Reference :default "/Game/VRE/Input/Actions/PrimaryGripLeft.PrimaryGripLeft"))
  (bind _leftmotioncontroller (Variables|Default|GetLeftMotionController))
  (bind _rightmotioncontroller (Variables|Default|GetRightMotionController))
  ;[0 1 0.1887] Grip
  (:Started
    (Grip|TrytoGetProps _leftmotioncontroller (Variables|Default|GetLPropsSphereCollision)) ; 从自身携带物品进行获取
    (Grip|TrytoGrabObject _leftmotioncontroller _rightmotioncontroller))
  (:Completed
    (Grip|DropAllGripObjects _leftmotioncontroller _rightmotioncontroller)))

(event Input|EnhancedActionEvents|EnhancedInputActionUseHeldObjectLeft
  (params (ActionValue :type Boolean) (ElapsedSeconds :type Float%20%28double-precision%29) (TriggeredSeconds :type Float%20%28double-precision%29) (InputAction :type Input%20Action%20Object%20Reference :default "/Game/VRE/Input/Actions/UseHeldObjectLeft.UseHeldObjectLeft"))
  (bind _rightmotioncontroller (Variables|Default|GetRightMotionController))
  (bind _leftmotioncontroller (Variables|Default|GetLeftMotionController))
  ;[1 0.4104 0] Trigger Used
  (:Started
    (TriggerUse|UseHeldObject _leftmotioncontroller _rightmotioncontroller true))
  (:Completed
    (TriggerUse|UseHeldObject _leftmotioncontroller _rightmotioncontroller false)))

(event Input|EnhancedActionEvents|EnhancedInputActionMotionControllerThumbLeft_Y
  (params (ActionValue :type Float%20%28double-precision%29) (ElapsedSeconds :type Float%20%28double-precision%29) (TriggeredSeconds :type Float%20%28double-precision%29) (InputAction :type Input%20Action%20Object%20Reference :default "/Game/VRE/Input/Actions/MotionControllerThumbLeft_Y.MotionControllerThumbLeft_Y"))
  (bind _vrreplicatedcamera (Variables|Default|GetVRReplicatedCamera))
  (bind _returnvalue (Math|Vector|GetForwardVector _vrreplicatedcamera))
  ;[1 1 1] Movement
  (:Triggered
    (Pawn|Input|AddMovementInput (Math|Vector|MakeVector (.x _returnvalue) (.y _returnvalue) 0.0) ActionValue false)))

(event Input|EnhancedActionEvents|EnhancedInputActionPrimaryGripRight
  (params (ActionValue :type Boolean) (ElapsedSeconds :type Float%20%28double-precision%29) (TriggeredSeconds :type Float%20%28double-precision%29) (InputAction :type Input%20Action%20Object%20Reference :default "/Game/VRE/Input/Actions/PrimaryGripRight.PrimaryGripRight"))
  (bind _leftmotioncontroller (Variables|Default|GetLeftMotionController))
  (bind _rightmotioncontroller (Variables|Default|GetRightMotionController))
  ;[0 1 0.1887] Grip
  (:Started
    (Grip|TrytoGetProps _rightmotioncontroller (Variables|Default|GetRPropsSphereCollision)) ; 从自身携带物品进行获取
    (Grip|TrytoGrabObject _rightmotioncontroller _leftmotioncontroller))
  (:Completed
    (Grip|DropAllGripObjects _rightmotioncontroller _leftmotioncontroller)))

(event EventBeginPlay
  ;[1 1 1] 记录初始手模型的相对变换
  (Variables|Grip|SetLHandOriginTransform (Transformation|GetRelativeTransform (Variables|Default|GetSKLeftHand)))
  (Variables|Grip|SetRHandOriginTransform (Transformation|GetRelativeTransform (Variables|Default|GetSKRightHand)))
  (Utilities|FlowControl|Delay 1.0 :!label _label) ; 确保角色重生后能正确获取到其Controller
  (bind _asbp_my_vrplayer_controller (Utilities|Casting|CastToBP_MyVRPlayerController (Game|GetInstigatorController))
    (:then
      (bind _output_get (Variables|Default|SetVRPlayerController _asbp_my_vrplayer_controller))
      (CallFunction|InitCharacterStatus _output_get))
    (:CastFailed
      (goto _label))))

(event Custom|PlayerDead
  (bind _vrreplicatedcamera (Variables|Default|GetVRReplicatedCamera))
  ;[1 0.1458 0.1458] 角色死亡
  (bind _returnvalue (Game|SpawnActorfromClass "/Game/MyVRProject/Blueprint/UI/BP_UIDeadBlack.BP_UIDeadBlack_C" (Transformation|GetWorldTransform _vrreplicatedcamera) "Undefined" 0 0))
  (Transformation|AttachComponentToComponent _returnvalue _vrreplicatedcamera "None" "KeepRelative" "KeepRelative" "KeepRelative" true)
  (bind _alpha (Timeline|时间轴 Play)
    (:Update
      (Default|DeadBlack _returnvalue (Math|Float|Lerp 0.0 1.0 _alpha)))
    (:Finished
      (Utilities|FlowControl|Delay 0.2)
      (Actor|DestroyActor))))

(event Game|Damage|EventAnyDamage
  (params (Damage :type Float%20%28single-precision%29) (DamageType :type Damage%20Type%20Object%20Reference) (InstigatedBy :type Controller%20Object%20Reference) (DamageCauser :type Actor%20Object%20Reference))
  (if (> (Variables|Default|GetCurrentHP) 0.0)
    (Variables|Default|SetCurrentHP Damage)))

(fn ConstructionScript)

(fn GetBoneTransform
  (params (Object :type Object%20Object%20Reference) (BoneName :type Name))
  (if (Utilities|Name|NotEqual(Name) BoneName "None")
    (bind _asscene_component (Utilities|Casting|CastToSceneComponent Object)
      (:then
        (return (Transformation|GetSocketTransform _asscene_component BoneName "RTS_World")))
      (:CastFailed
        (bind _asskeletal_mesh_actor (Utilities|Casting|CastToSkeletalMeshActor Object)
          (:then
            (return (Transformation|GetSocketTransform (Variables|/Script/Engine.SkeletalMeshActor|GetSkeletalMeshComponent _asskeletal_mesh_actor) BoneName "RTS_World")))
          (:CastFailed
            _)))))
  (return ""))

(fn DropAllGripObjects
  (params (CallingMotionController :type Grip%20Motion%20Controller%20Component%20Object%20Reference) (OtherMotionController :type Grip%20Motion%20Controller%20Component%20Object%20Reference))
  (bind _skrighthand (Variables|Default|GetSKRightHand))
  (bind _sklefthand (Variables|Default|GetSKLeftHand))
  (if (Class|GripMotionControllerComponent|HasGrippedObjects CallingMotionController)
    (bind _griparray (Class|GripMotionControllerComponent|GetAllGrips CallingMotionController))
    (for _array_element _griparray
      (bind _returnvalue (Class|VRGripInterface|GripMovementReplicationType(Message) (.GrippedObject (Utilities|Struct|BreakBPActorGripInformation _array_element))))
      (if (Grip|IsALocalGrip _returnvalue)
        (CallFunction|TrytoDropClient CallingMotionController (.GrippedObject (Utilities|Struct|BreakBPActorGripInformation _array_element)) (.GripID (Utilities|Struct|BreakBPActorGripInformation _array_element)) false)
        (else
          (CallFunction|TrytoDropServer CallingMotionController (.GrippedObject (Utilities|Struct|BreakBPActorGripInformation _array_element)) (.GripID (Utilities|Struct|BreakBPActorGripInformation _array_element)) false)))
      (if (Utilities|Enum|Equal(Enum) (Class|GripMotionControllerComponent|GetHandType CallingMotionController) "Left")
        (Variables|Grip|SetLHandSocketPose "")
        (Transformation|AttachComponentToComponent _sklefthand (Variables|Default|GetLeftMotionController) "None" "SnapToTarget" "KeepWorld" "KeepWorld" true)
        (Transformation|SetRelativeTransform _sklefthand (Variables|Grip|GetLHandOriginTransform) false false)
        (Transformation|AttachComponentToComponent (Variables|Default|GetLAttachmentProxy) (Variables|Default|GetLeftMotionController) "None" "KeepWorld" "KeepWorld" "KeepWorld" true)
        (else
          (Variables|Grip|SetRHandSocketPose "")
          (Transformation|AttachComponentToComponent _skrighthand (Variables|Default|GetRightMotionController) "None" "SnapToTarget" "KeepWorld" "KeepWorld" true)
          (Transformation|SetRelativeTransform _skrighthand (Variables|Grip|GetRHandOriginTransform) false false)
          (Transformation|AttachComponentToComponent (Variables|Default|GetRAttachmentProxy) (Variables|Default|GetRightMotionController) "None" "KeepWorld" "KeepWorld" "KeepWorld" true))))
    (else
      (bind (_grip _returnvalue_2) (Class|GripMotionControllerComponent|GetIsSecondaryAttachment OtherMotionController CallingMotionController))
      (if _returnvalue_2
        (bind _returnvalue_3 (Class|VRGripInterface|GripMovementReplicationType(Message) (.GrippedObject (Utilities|Struct|BreakBPActorGripInformation _grip))))
        (if (Grip|IsALocalGrip _returnvalue_3)
          (CallFunction|TrytoDropClient OtherMotionController (.GrippedObject (Utilities|Struct|BreakBPActorGripInformation _grip)) (.GripID (Utilities|Struct|BreakBPActorGripInformation _grip)) true)
          (else
            (CallFunction|TrytoDropServer OtherMotionController (.GrippedObject (Utilities|Struct|BreakBPActorGripInformation _grip)) (.GripID (Utilities|Struct|BreakBPActorGripInformation _grip)) true)))
        (if (Utilities|Enum|Equal(Enum) (Class|GripMotionControllerComponent|GetHandType CallingMotionController) "Left")
          (Variables|Grip|SetLHandSocketPose "")
          (Transformation|AttachComponentToComponent _sklefthand (Variables|Default|GetLeftMotionController) "None" "SnapToTarget" "KeepWorld" "KeepWorld" true)
          (Transformation|SetRelativeTransform _sklefthand (Variables|Grip|GetLHandOriginTransform) false false)
          (Transformation|AttachComponentToComponent (Variables|Default|GetLAttachmentProxy) (Variables|Default|GetLeftMotionController) "None" "KeepWorld" "KeepWorld" "KeepWorld" true)
          (else
            (Variables|Grip|SetRHandSocketPose "")
            (Transformation|AttachComponentToComponent _skrighthand (Variables|Default|GetRightMotionController) "None" "SnapToTarget" "KeepWorld" "KeepWorld" true)
            (Transformation|SetRelativeTransform _skrighthand (Variables|Grip|GetRHandOriginTransform) false false)
            (Transformation|AttachComponentToComponent (Variables|Default|GetRAttachmentProxy) (Variables|Default|GetRightMotionController) "None" "KeepWorld" "KeepWorld" "KeepWorld" true)))))))

(fn GetNearestGripObject
  (params (CallingMotionController :type Grip%20Motion%20Controller%20Component%20Object%20Reference))
  (bind _returnvalue (Transformation|GetWorldLocation CallingMotionController))
  (bind (_outhits _returnvalue_2) (Collision|MultiSphereTraceByChannel _returnvalue _returnvalue 8.0 "TraceTypeQuery1" false 0 "None"))
  (if _returnvalue_2
    (bind (_gripobject _worldtransform _griplocation _bonename) (Grip|SelectGripObjectfromHits _outhits CallingMotionController))
    (Utilities|IsValid _gripobject
      (:Is%20Valid
        (return _gripobject _worldtransform _griplocation _bonename))
      (:Is%20Not%20Valid
        _)))
  (return 0 "" "0, 0, 0" "None"))

(fn SelectGripObjectfromHits
  (params (ObjectHits :type Array%20of%20Hit%20Result%20Structures) (CallingMotionController :type Grip%20Motion%20Controller%20Component%20Object%20Reference))
  (for _array_element ObjectHits
    (bind (_isbestprio _newgrippriority _newobject _hitlocation _hitbonename _worldtransform) (Grip|CheckBestPrioObject _array_element CallingMotionController (LocalVariables|GetBestGripPriority)))
    (if _isbestprio
      (LocalVariables|SetBestGripPriority _newgrippriority)
      (LocalVariables|SetLObjectToGrip _newobject)
      (LocalVariables|SetLGripLocation _hitlocation)
      (LocalVariables|SetLBoneName _hitbonename)
      (LocalVariables|SetLWorldTransform _worldtransform)))
  (return (LocalVariables|GetLObjectToGrip) (LocalVariables|GetLWorldTransform) (LocalVariables|GetLGripLocation) (LocalVariables|GetLBoneName)))

(fn TrytoGrabObject
  (params (CallingMotionController :type Grip%20Motion%20Controller%20Component%20Object%20Reference) (OtherMotionController :type Grip%20Motion%20Controller%20Component%20Object%20Reference))
  (if (not (Class|GripMotionControllerComponent|HasGrippedObjects CallingMotionController))
    (bind (_gripobject _objectworldtransform _griplocation _bonename) (Grip|GetNearestGripObject CallingMotionController))
    (Utilities|IsValid _gripobject
      (:Is%20Valid
        (LocalVariables|SetObjectToGrip _gripobject)
        (LocalVariables|SetObjectTransform _objectworldtransform)
        (LocalVariables|SetGripLocation _griplocation)
        (LocalVariables|SetBoneName _bonename)
        (bind (_holdingcontrollers _bisheld) (Class|VRGripInterface|IsHeld(Message) (LocalVariables|GetObjectToGrip)))
        (if _bisheld
          (if (Grip|CheckSecondaryGrip _holdingcontrollers (LocalVariables|GetObjectToGrip) OtherMotionController)
            (bind (_isslotrelativegrip _wordtransform _gripslotname) (Grip|CheckGripSlotinRange (LocalVariables|GetObjectToGrip) (LocalVariables|GetGripLocation) true CallingMotionController "VRGripS" (LocalVariables|GetBoneName) (LocalVariables|GetObjectTransform)))
            (bind _returnvalue (Class|VRGripInterface|GripMovementReplicationType(Message) (LocalVariables|GetObjectToGrip)))
            (if (Grip|IsALocalGrip _returnvalue)
              (CallFunction|TrytoGrabClient CallingMotionController OtherMotionController (LocalVariables|GetObjectToGrip) _wordtransform _isslotrelativegrip _gripslotname (LocalVariables|GetBoneName) true)
              (else
                (CallFunction|TrytoGrabServer CallingMotionController OtherMotionController (LocalVariables|GetObjectToGrip) _wordtransform _isslotrelativegrip _gripslotname (LocalVariables|GetBoneName) true)))
            (else
              (bind _returnvalue_2 (Class|VRGripInterface|AllowsMultipleGrips(Message) (LocalVariables|GetObjectToGrip)))
              (if _returnvalue_2
                (bind (_isslotrelativegrip_2 _wordtransform_2 _gripslotname_2) (Grip|CheckGripSlotinRange (LocalVariables|GetObjectToGrip) (LocalVariables|GetGripLocation) false CallingMotionController "VRGripP" (LocalVariables|GetBoneName) (LocalVariables|GetObjectTransform) :!label _label))
                (bind _returnvalue_3 (Class|VRGripInterface|GripMovementReplicationType(Message) (LocalVariables|GetObjectToGrip)))
                (if (Grip|IsALocalGrip _returnvalue_3)
                  (CallFunction|TrytoGrabClient CallingMotionController OtherMotionController (LocalVariables|GetObjectToGrip) _wordtransform_2 _isslotrelativegrip_2 _gripslotname_2 (LocalVariables|GetBoneName) false)
                  (else
                    (CallFunction|TrytoGrabServer CallingMotionController OtherMotionController (LocalVariables|GetObjectToGrip) _wordtransform_2 _isslotrelativegrip_2 _gripslotname_2 (LocalVariables|GetBoneName) false))))))
          (else
            (goto _label)))))))

(fn CheckGripSlotinRange
  (params (ObjectToCheck :type Object%20Object%20Reference) (GripLocation :type Vector) (isSecondarySlot :type Boolean) (CallingMontionController :type Grip%20Motion%20Controller%20Component%20Object%20Reference) (OverridePrefix :type Name) (OptionalBoneName :type Name) (ObjectTransform :type Transform))
  (bind _bonetransform (Grip|GetBoneTransform ObjectToCheck OptionalBoneName))
  (bind _returnvalue (== OptionalBoneName ""))
  (bind _returnvalue_2 (select _returnvalue ObjectTransform _bonetransform))
  (bind (_bhadslotinrange _slotworldtransform _slotname) (Class|VRGripInterface|ClosestGripSlotinRange(Message) ObjectToCheck GripLocation isSecondarySlot CallingMontionController OverridePrefix))
  (if _bhadslotinrange
    ;[1 1 1] 处理HandSocket动画快照
    (bind _returnvalue_3 (Class|HandSocketComponent|GetHandSocketComponentfromObject ObjectToCheck _slotname))
    (Utilities|IsValid _returnvalue_3
      (:Is%20Valid
        (bind (_posesnapshot _returnvalue_4) (Class|HandSocketComponent|GetBlendedPoseSnapShot _returnvalue_3 (.SKHand (Grip|GetControllerHandMesh CallingMontionController)) false false))
        (if _returnvalue_4
          (if (Utilities|Enum|Equal(Enum) (Class|GripMotionControllerComponent|GetHandType CallingMontionController) "Left")
            (Variables|Grip|SetLHandSocketPose _posesnapshot)
            (else
              (Variables|Grip|SetRHandSocketPose _posesnapshot))))
        (return true (select isSecondarySlot (Class|GripMotionControllerComponent|ConverttoGripRelativeTransform _returnvalue_2 _slotworldtransform) (Class|KismetMathLibrary|ConvertTransformtoRelative _slotworldtransform _returnvalue_2)) _slotname)))
    (else
      (return false ObjectTransform "None"))))

(fn CheckBestPrioObject
  (params (HitObjectCheck :type Hit%20Result%20Structure) (CallingController :type Grip%20Motion%20Controller%20Component%20Object%20Reference) (DefaultPriority :type Byte))
  (bind (_bblockinghit _binitialoverlap _time _distance _location _impactpoint _normal _impactnormal _physmat _hitactor _hitcomponent _hitbonename) (Collision|BreakHitResult HitObjectCheck))
  (if (Utilities|DoesObjectImplementInterface _hitcomponent "/Script/VRExpansionPlugin.VRGripInterface")
    (bind _returnvalue (Class|VRGripInterface|DenyGripping(Message) _hitcomponent CallingController))
    (if _returnvalue
      _
      (else
        (bind _returnvalue_2 (Class|VRGripInterface|AdvancedGripSettings(Message) _hitcomponent))
        (if (> (.grippriority _returnvalue_2) DefaultPriority)
          (return true (.grippriority _returnvalue_2) _hitcomponent _location _hitbonename (Transformation|GetWorldTransform _hitcomponent))
          (else
            _))))
    (elif (Utilities|DoesObjectImplementInterface _hitactor "/Script/VRExpansionPlugin.VRGripInterface")
      (bind _returnvalue_3 (Class|VRGripInterface|DenyGripping(Message) _hitactor CallingController))
      (if _returnvalue_3
        _
        (else
          (bind _returnvalue_4 (Class|VRGripInterface|AdvancedGripSettings(Message) _hitactor))
          (if (> (.grippriority _returnvalue_4) DefaultPriority)
            (return true (.grippriority _returnvalue_4) _hitactor _location _hitbonename (Transformation|GetActorTransform _hitactor))
            (else
              _))))))
  (return false 0 0 "0, 0, 0" "None" ""))

(fn CheckSecondaryGrip
  (params (HoldingControllers :type Array%20of%20BP%20Grip%20Pair%20Structures) (ObjectToCheck :type Object%20Object%20Reference) (OtherMotionController :type Grip%20Motion%20Controller%20Component%20Object%20Reference))
  (bind _returnvalue (Class|VRGripInterface|SecondaryGripType(Message) ObjectToCheck))
  (return (and (Utilities|Enum|NotEqual(Enum) _returnvalue "SG_None") (== (.HoldingController (Utilities|Struct|BreakBPGripPair (Utilities|Array|Get(acopy) HoldingControllers))) OtherMotionController))))

(fn GetControllerHandMesh
  (params (CallingMotionController :type Grip%20Motion%20Controller%20Component%20Object%20Reference))
  (if (Utilities|Enum|Equal(Enum) (Class|GripMotionControllerComponent|GetHandType CallingMotionController) "Left")
    (return (Variables|Default|GetSKLeftHand) false)
    (else
      (return (Variables|Default|GetSKRightHand) true))))

(fn SlotGripHandAnimAttachment
  (params (ObjectToAttachment :type Object%20Object%20Reference) (ControllerSKHand :type Skeletal%20Mesh%20Component%20Object%20Reference) (SlotName :type Name) (isRightHand :type Boolean))
  (bind _rattachmentproxy (Variables|Default|GetRAttachmentProxy))
  (bind _rattachmentproxy_2 (Variables|Default|GetRAttachmentProxy))
  (bind _lattachmentproxy (Variables|Default|GetLAttachmentProxy))
  (bind _lattachmentproxy_2 (Variables|Default|GetLAttachmentProxy))
  (bind _returnvalue (Class|HandSocketComponent|GetHandSocketComponentfromObject ObjectToAttachment SlotName))
  (Utilities|IsValid _returnvalue
    (:Is%20Valid
      (LocalVariables|SetHandSocketCompnent _returnvalue)
      (if isRightHand
        (bind _asprimitive_component (Utilities|Casting|CastToPrimitiveComponent ObjectToAttachment)
          (:then
            (Transformation|AttachComponentToComponent _rattachmentproxy_2 _asprimitive_component "None" "SnapToTarget" "SnapToTarget" "KeepWorld" true))
          (:CastFailed
            (bind _asactor (Utilities|Casting|CastToActor ObjectToAttachment))
            (Transformation|AttachComponentToComponent _rattachmentproxy_2 (Variables|/Script/Engine.Actor|GetRootComponent _asactor) "None" "SnapToTarget" "SnapToTarget" "KeepWorld" true)))
        (bind _returnvalue_2 (Class|HandSocketComponent|GetMeshRelativeTransform (LocalVariables|GetHandSocketCompnent) isRightHand false false))
        (Transformation|SetRelativeLocationAndRotation _rattachmentproxy (.location _returnvalue_2) (.rotation _returnvalue_2) false false)
        (Transformation|AttachComponentToComponent ControllerSKHand _rattachmentproxy "None" "SnapToTarget" "SnapToTarget" "KeepWorld" true)
        (else
          (bind _asprimitive_component_2 (Utilities|Casting|CastToPrimitiveComponent ObjectToAttachment)
            (:then
              (Transformation|AttachComponentToComponent _lattachmentproxy _asprimitive_component_2 "None" "SnapToTarget" "SnapToTarget" "KeepWorld" true))
            (:CastFailed
              (bind _asactor_2 (Utilities|Casting|CastToActor ObjectToAttachment))
              (Transformation|AttachComponentToComponent _lattachmentproxy (Variables|/Script/Engine.Actor|GetRootComponent _asactor_2) "None" "SnapToTarget" "SnapToTarget" "KeepWorld" true)))
          (bind _returnvalue_3 (Class|HandSocketComponent|GetMeshRelativeTransform (LocalVariables|GetHandSocketCompnent) isRightHand false false))
          (Transformation|SetRelativeLocationAndRotation _lattachmentproxy_2 (.location _returnvalue_3) (.rotation _returnvalue_3) false false)
          (Transformation|AttachComponentToComponent ControllerSKHand _lattachmentproxy_2 "None" "SnapToTarget" "SnapToTarget" "KeepWorld" true))))))

(fn UseHeldObject
  (params (CallingMotionController :type Grip%20Motion%20Controller%20Component%20Object%20Reference) (OtherMotionController :type Grip%20Motion%20Controller%20Component%20Object%20Reference) (isUsed :type Boolean))
  (bind (_grip _returnvalue) (Class|GripMotionControllerComponent|GetIsSecondaryAttachment OtherMotionController CallingMotionController))
  (if (not _returnvalue)
    (bind _griparray (Class|GripMotionControllerComponent|GetAllGrips CallingMotionController))
    (for _array_element _griparray
      (Utilities|IsValid (.GrippedObject (Utilities|Struct|BreakBPActorGripInformation _array_element))
        (:Is%20Valid
          (if isUsed
            (bind _asvrgrip_interface (Utilities|Casting|CastToVRGripInterface (.GrippedObject (Utilities|Struct|BreakBPActorGripInformation _array_element))))
            (Class|VRGripInterface|OnUsed _asvrgrip_interface)
            (else
              (bind _asvrgrip_interface_2 (Utilities|Casting|CastToVRGripInterface (.GrippedObject (Utilities|Struct|BreakBPActorGripInformation _array_element))))
              (Class|VRGripInterface|OnEndUsed _asvrgrip_interface_2))))))
    (elif isUsed
      (Class|VRGripInterface|OnSecondaryUsed(Message) (.GrippedObject (Utilities|Struct|BreakBPActorGripInformation _grip)))
      (else
        (Class|VRGripInterface|OnEndSecondaryUsed(Message) (.GrippedObject (Utilities|Struct|BreakBPActorGripInformation _grip)))))))

(fn InitCharacterStatus
  (params (PlayerController :type BP%20My%20VR%20Player%20Controller%20Object%20Reference))
  (bind _sklefthand (Variables|Default|GetSKLeftHand))
  (Variables|Default|SetCurrentHP (.maxhp (Variables|Default|GetCharcAttribute)))
  (Variables|Default|SetTags (Variables|Default|GetPlayerTags)) ; 标记角色Tag，用于AI识别
  (Class|HeadMountedDisplayFunctionLibrary|SetTrackingOrigin "Floor")
  ;[1 0.3012 0.4212] 角色状态的UI信息
  (Default|SpawnUIWidget PlayerController (Transformation|GetWorldTransform _sklefthand) _sklefthand)
  (Default|UpdateHPPercentUI PlayerController (Variables|Default|GetCurrentHP) (.maxhp (Variables|Default|GetCharcAttribute)))
  (Default|UpdateBulltesNumUI PlayerController 0 (Variables|Gun|GetTotalBullets)))

(fn GrabObject
  (params (CallingMotionController :type Grip%20Motion%20Controller%20Component%20Object%20Reference) (OtherMotionController :type Grip%20Motion%20Controller%20Component%20Object%20Reference) (ObjectToGrip :type Object%20Object%20Reference) (ObjectTransform :type Transform%20%28by%20ref%29) (isSlotRelativeGrip :type Boolean) (SlotName :type Name) (BoneName :type Name) (isSecondaryGrip :type Boolean))
  (bind (_skhand _isrighthand) (Grip|GetControllerHandMesh CallingMotionController))
  (if isSlotRelativeGrip
    (Grip|SlotGripHandAnimAttachment ObjectToGrip _skhand SlotName _isrighthand))
  (if isSecondaryGrip
    (Class|GripMotionControllerComponent|AddSecondaryAttachmentPoint OtherMotionController ObjectToGrip CallingMotionController ObjectTransform isSlotRelativeGrip 0.25 isSlotRelativeGrip SlotName)
    (else
      (Class|GripMotionControllerComponent|GripObjectbyInterface CallingMotionController ObjectToGrip ObjectTransform isSlotRelativeGrip BoneName SlotName isSlotRelativeGrip))))

(fn OnRepCurrentHP
  (bind _currenthp (Variables|Default|GetCurrentHP))
  (if (<= _currenthp 0.0)
    (CallFunction|UpdateHPWidget 0.0)
    (Utilities|Array|RemoveItem (Variables|Default|GetTags) "Player")
    (CallFunction|PlayerDead)
    (else
      (CallFunction|UpdateHPWidget _currenthp))))

(fn IsALocalGrip
  (params (GripRepType :type EGripMovementReplicationSettings%20Enum :default "KeepOriginalMovement"))
  (return (or (Utilities|Enum|Equal(Enum) GripRepType "ClientSide_Authoritive") (Utilities|Enum|Equal(Enum) GripRepType "ClientSide_Authoritive_NoRep"))))

(fn TrytoGetProps
  (params (CallingMotionController :type Grip%20Motion%20Controller%20Component%20Object%20Reference) (PropsSphereCollision :type Sphere%20Component%20Object%20Reference))
  (bind _gunammobullets (Variables|Gun|GetGunAmmoBullets))
  (if (and (Class|PrimitiveComponent|IsOverlappingComponent PropsSphereCollision (Variables|Default|GetPropsBox)) (> (Variables|Gun|GetTotalBullets) 0))
    (bind _vrplayercontroller (Variables|Default|GetVRPlayerController)
      (:then
        (Default|SpawnPropsServer _vrplayercontroller "/Game/MyVRProject/Blueprint/Weapons/AR4/BP_AR4_Ammo.BP_AR4_Ammo_C" (Class|GripMotionControllerComponent|GetPivotTransformBP CallingMotionController))
        (Audio|PlaySoundatLocation "/Game/MyVRProject/Assets/Sounds/Gun/弹夹取出.弹夹取出" (Class|GripMotionControllerComponent|GetPivotLocationBP CallingMotionController) "0, 0, 0" 1.0 1.0 0.0 0 0 0 0)
        (Variables|Gun|SetTotalBullets (Math|Integer|SelectInt 0 (- (Variables|Gun|GetTotalBullets) _gunammobullets) (< (Variables|Gun|GetTotalBullets) _gunammobullets)))
        (CallFunction|UpdateBulletNumWidget))
      (:else))))

(fn DropObject
  (params (MotionController :type Grip%20Motion%20Controller%20Component%20Object%20Reference) (ObjectToDrop :type Object%20Object%20Reference) (GripIDToDrop :type Byte) (isSecondary :type Boolean))
  (if isSecondary
    (Class|GripMotionControllerComponent|RemoveSecondaryAttachmentPoint MotionController ObjectToDrop 0.25)
    (else
      (Class|GripMotionControllerComponent|DropObjectbyInterface MotionController ObjectToDrop GripIDToDrop "0, 0, 0" "0, 0, 0"))))

(fn IsOverWidgetUse
  (params (CallingWidgetInteraction :type Widget%20Interaction%20Component%20Object%20Reference) (isPressed :type Boolean))
  (Utilities|IsValid CallingWidgetInteraction
    (:Is%20Valid
      (if (or (Class|WidgetInteractionComponent|IsOverInteractableWidget CallingWidgetInteraction) (Class|WidgetInteractionComponent|IsOverFocusableWidget CallingWidgetInteraction))
        (if isPressed
          (Class|WidgetInteractionComponent|PressPointerKey CallingWidgetInteraction "LeftMouseButton")
          (else
            (Class|WidgetInteractionComponent|ReleasePointerKey CallingWidgetInteraction "LeftMouseButton")))
        (return true)
        (else
          _)))
    (:Is%20Not%20Valid
      _))
  (return false))