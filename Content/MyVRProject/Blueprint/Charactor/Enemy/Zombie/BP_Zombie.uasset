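; Zombie enemy character that feeds its AI controller's blackboard and handles melee attacks and damage.
; BeginPlay sets the patrol and scream keys, and an attack-range sphere toggles another key as the player enters, clearing it on any end overlap.
; AGR CombatManager events damage the player once per swing and raise walk speed during attacks for a charging lunge.
; Incoming damage reduces HP until death; a low-health stagger exists but is disconnected.
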(event EventBeginPlay
  (|CallParentFunction)
  ;[1 1 1] 丧尸的行为设置
  (bind _asaic_zombie_controller (Utilities|Casting|CastToAIC_ZombieController (Pawn|GetController)))
  (AI|Components|Blackboard|SetValueasBool (AI|GetBlackboard _asaic_zombie_controller) (Variables|Default|GetPatrol) (Variables|Default|GetNeedPatrol))
  (AI|Components|Blackboard|SetValueasBool (AI|GetBlackboard _asaic_zombie_controller) (Variables|Default|GetScream) (Variables|Default|GetShouldScream)))

(event Collision|EventActorBeginOverlap
  (params (OtherActor :type Actor%20Object%20Reference))
  (|CallParentFunction OtherActor) ; 此节点被禁用，将不会被调用。\n从引脚连出引线来编译功能。
)

(event EventTick
  (params (DeltaSeconds :type Float%20%28single-precision%29))
  (|CallParentFunction DeltaSeconds) ; 此节点被禁用，将不会被调用。\n从引脚连出引线来编译功能。
)

(event OnEndAttack(AGR_CombatManager)
  ;[1 1 1] AGR插件：攻击判定，应用伤害
  ;;[1 0.2344 0.2344] 攻击检测开始时，清空ignore数组。
  ;; 攻击时提高移动速度实现蓄力攻击，增强检测范围。
  (CallFunction|UpdateMaxWalkSpeed 5e+02))

(event OnComponentBeginOverlap(AttackSphereRange)
  (params (OverlappedComponent :type Primitive%20Component%20Object%20Reference) (OtherActor :type Actor%20Object%20Reference) (OtherComp :type Primitive%20Component%20Object%20Reference) (OtherBodyIndex :type Integer) (bFromSweep :type Boolean) (SweepResult :type Hit%20Result%20Structure%20%28by%20ref%29))
  ;[0.8287 0.1928 1] 根据AttackSphereRange检测是否在攻击范围内
  (if (Actor|ActorHasTag OtherActor "Player")
    (bind _asaic_zombie_controller (Utilities|Casting|CastToAIC_ZombieController (Pawn|GetController)))
    (AI|Components|Blackboard|SetValueasBool (AI|GetBlackboard _asaic_zombie_controller) (Variables|Default|GetBBKeyName) true)))

(event OnComponentEndOverlap(AttackSphereRange)
  (params (OverlappedComponent :type Primitive%20Component%20Object%20Reference) (OtherActor :type Actor%20Object%20Reference) (OtherComp :type Primitive%20Component%20Object%20Reference) (OtherBodyIndex :type Integer))
  ;[0.8287 0.1928 1] 根据AttackSphereRange检测是否在攻击范围内
  (bind _asaic_zombie_controller (Utilities|Casting|CastToAIC_ZombieController (Pawn|GetController)))
  (AI|Components|Blackboard|SetValueasBool (AI|GetBlackboard _asaic_zombie_controller) (Variables|Default|GetBBKeyName) false))

(event OnAttackHitEvent(AGR_CombatManager)
  (params (Hit :type Hit%20Result%20Structure) (Mesh :type Primitive%20Component%20Object%20Reference))
  (bind _hitactor (Collision|BreakHitResult Hit))
  (bind _agr_combatmanager (Variables|Default|GetAGR_CombatManager))
  (bind _ignoredactors (Variables|/Script/AGRPRO.AGR_CombatManager|GetIgnoredActors _agr_combatmanager))
  ;[1 1 1] AGR插件：攻击判定，应用伤害
  (if (not (Utilities|Array|ContainsItem _ignoredactors _hitactor))
    (Utilities|Array|AddUnique _ignoredactors _hitactor)
    (if (Actor|ActorHasTag _hitactor "Player")
      (Game|Damage|ApplyDamage _hitactor (.damage (Variables|Default|GetCharAttribute)) 0 0))))

(event OnStartAttack(AGR_CombatManager)
  ;[1 1 1] AGR插件：攻击判定，应用伤害
  ;;[1 0.2344 0.2344] 攻击检测开始时，清空ignore数组。
  ;; 攻击时提高移动速度实现蓄力攻击，增强检测范围。
  (Class|AGRCombatManager|RefreshIgnoredActors (Variables|Default|GetAGR_CombatManager))
  (CallFunction|UpdateMaxWalkSpeed 8e+02))

(event Game|Damage|EventAnyDamage
  (params (Damage :type Float%20%28single-precision%29) (DamageType :type Damage%20Type%20Object%20Reference) (InstigatedBy :type Controller%20Object%20Reference) (DamageCauser :type Actor%20Object%20Reference))
  (if (not (Variables|Default|GetDeath))
    (CallFunction|GetHPDamage Damage)))

(fn ConstructionScript
  (|CallParentFunction))

(fn UpdateRotDirecition
  (bind _returnvalue (Pawn|GetControlRotation :!class /Script/Engine.Pawn))
  (bind _returnvalue_2 (Transformation|GetVelocity))
  (bind _returnvalue_3 (Class|KismetAnimationLibrary|CalculateDirection _returnvalue_2 _returnvalue))
  (Development|PrintString (Utilities|String|ToString(Float) _returnvalue_3))
  (return _returnvalue_3))