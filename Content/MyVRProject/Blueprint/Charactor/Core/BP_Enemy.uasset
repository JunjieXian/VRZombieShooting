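; BP_Enemy is an enemy character Blueprint that handles health, damage and death.
; On BeginPlay it fills HP from its attribute data and registers its mesh with AGRCombatManager for complex box tracing.
; GetHPDamage subtracts HP while alive, and RepNotifies chain HP depletion into Death, which ignores Pawn collision, detaches the controller and disables movement.
; A helper function sets max walk speed.
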(event EventBeginPlay
  (CallFunction|InitCharacterState))

(event Collision|EventActorBeginOverlap
  (params (OtherActor :type Actor%20Object%20Reference)))

(event EventTick
  (params (DeltaSeconds :type Float%20%28single-precision%29)))

(fn ConstructionScript)

(fn UpdateMaxWalkSpeed
  (params (Max%20Walk%20Speed :type Float%20%28single-precision%29))
  (Variables|/Script/Engine.CharacterMovementComponent|SetMaxWalkSpeed (Variables|Character|GetCharacterMovement) Max%20Walk%20Speed))

(fn GetHPDamage
  (params (Damage :type Float%20%28double-precision%29))
  (if (not (Variables|CharactorDefaultStatus|GetDeath))
    (Variables|CharactorDefaultStatus|SetCurrentHP (- (Variables|CharactorDefaultStatus|GetCurrentHP) Damage))))

(fn InitCharacterState
  (Variables|CharactorDefaultStatus|SetCurrentHP (.maxhp (Variables|CharactorDefaultStatus|GetCharAttribute)))
  (Class|AGRCombatManager|AddTraceMesh (Variables|Default|GetAGR_CombatManager) (Variables|Character|GetMesh) "ComplexBoxTrace"))

(fn OnRepCurrentHP
  (if (<= (Variables|CharactorDefaultStatus|GetCurrentHP) 0.0)
    (Variables|CharactorDefaultStatus|SetDeath true)))

(fn OnRepDeath
  (if (Variables|CharactorDefaultStatus|GetDeath)
    (Collision|SetCollisionResponsetoChannel (Variables|Collision|GetCapsuleComponent) "ECC_Pawn" "ECR_Ignore")
    (Class|Pawn|DetachfromControllerPendingDestroy)
    (Pawn|Components|CharacterMovement|DisableMovement (Variables|Character|GetCharacterMovement))))