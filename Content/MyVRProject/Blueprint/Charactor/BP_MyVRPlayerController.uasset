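; BP_MyVRPlayerController is the VR player controller handling input setup, status UI, respawning, prop spawning and session exit.
; It adds the input mapping context on BeginPlay and can spawn a status actor above the left hand, forwarding HP and bullet updates to it.
; UnPossess triggers a respawn through BP_MyVRGameMode.
; Prop spawning chains server to multicast events, and exiting destroys the session before opening the main menu.
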(event Custom|ExitSession
  ;[1 1 1] 退出联机
  (|DestroySession self
    (:OnSuccess
      (Game|OpenLevel(byObjectReference) "/Game/MyVRProject/Map/MainMenuMap.MainMenuMap"))))

(event Custom|RespawnPlayer_Server
  (params (SpawnTransform :type Transform))
  ;[0.1514 1 0.1329] 重生角色并控制
  (bind _asbp_my_vrgame_mode (Utilities|Casting|CastToBP_MyVRGameMode (Game|GetGameMode)))
  (Default|RespawnPlayer _asbp_my_vrgame_mode self SpawnTransform))

(event Custom|SpawnUIWidget
  (params (SpawnTransform :type Transform) (AttachCompParent :type Scene%20Component%20Object%20Reference))
  ;[1 0.2737 0.3736] 玩家状态信息UI
  (bind _returnvalue (Game|SpawnActorfromClass "/Game/MyVRProject/Blueprint/UI/BP_UICharStatus.BP_UICharStatus_C" SpawnTransform "Undefined" (Game|Player|GetPlayerPawn 0) 0))
  (bind _output_get (Variables|Default|SetPlayerStatusUI _returnvalue))
  (Transformation|AttachComponentToComponent _output_get AttachCompParent "None" "SnapToTarget" "SnapToTarget" "KeepRelative" true)
  (Transformation|SetActorRelativeTransform _output_get (Variables|Default|GetUIWidgtRelativeTransform) false false) ; 位于左手上方
)

(event Custom|UpdateHPPercentUI
  (params (CurrentHP :type Float%20%28double-precision%29) (MaxHP :type Float%20%28double-precision%29))
  ;[1 0.2737 0.3736] 玩家状态信息UI
  (bind _playerstatusui (Variables|Default|GetPlayerStatusUI)
    (:then
      (Default|UpdateHPPercent _playerstatusui CurrentHP MaxHP))
    (:else)))

(event Custom|UpdateBulltesNumUI
  (params (CurrentBullets :type Integer) (TotalBullets :type Integer))
  ;[1 0.2737 0.3736] 玩家状态信息UI
  (bind _playerstatusui (Variables|Default|GetPlayerStatusUI)
    (:then
      (Default|UpdateBulletsNum _playerstatusui CurrentBullets TotalBullets))
    (:else)))

(event Custom|SpawnProps_Server
  (params (PropsClass :type Actor%20Class%20Reference) (SpawnTransform :type Transform))
  ;[1 1 1] 道具生成
  (CallFunction|SpawnPropsMulti PropsClass SpawnTransform))

(event Custom|SpawnProps_Multi
  (params (PropsClass :type Actor%20Class%20Reference) (SpawnTransform :type Transform))
  ;[1 1 1] 道具生成
  (CallFunction|SpawnProps PropsClass SpawnTransform))

(event Custom|SpawnProps
  (params (PropsClass :type Actor%20Class%20Reference) (SpawnTransform :type Transform))
  ;[1 1 1] 道具生成
  (Game|SpawnActorfromClass PropsClass SpawnTransform "Undefined" 0 0))

(event EventBeginPlay
  (bind _returnvalue (PlayerController|LocalPlayerSubsystems|GetEnhancedInputLocalPlayerSubsystem))
  (Utilities|IsValid _returnvalue
    (:Is%20Valid
      (Input|AddMappingContext _returnvalue "/Game/VRE/Input/VREInputMappingContext.VREInputMappingContext" 0 "(bIgnoreAllPressedKeysUntilRelease=True,bForceImmediately=False)"))))

(event EventUnPossess
  (params (UnpossessedPawn :type Pawn%20Object%20Reference))
  ;[0.1514 1 0.1329] 重生角色并控制
  (CallFunction|RespawnPlayerServer (Variables|Default|GetReSpawn%20Transform)))

(fn ConstructionScript)