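; Bullet actor for VR weapons that resolves its impact, then destroys itself.
; Hits relay through server and multicast events into a shared handler, so damage logic sits on the multicast path.
; Enemies take point damage, reported to AI damage sensing with the VR character as instigator.
; Other targets get an impulse if simulating physics, an attached random hole decal and Niagara impact effect; blood feedback is an unconnected TODO.
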(event Custom|BulletHit
  (params (HitActor :type Object%20Object%20Reference) (Hit%20Comp :type Primitive%20Component%20Object%20Reference) (HitLocation :type Vector%20%28by%20ref%29) (HitNormal :type Vector) (HitInfo :type Hit%20Result%20Structure%20%28by%20ref%29))
  (bind _returnvalue (* HitNormal -1.0))
  (bind _vrcharacter (Variables|Default|GetVRCharacter))
  (bind _returnvalue_2 (Math|Rotator|MakeRotfromX _returnvalue))
  (Variables|Default|SetHit%20Comp Hit%20Comp)
  (bind _asbp_enemy (Utilities|Casting|CastToBP_Enemy HitActor)
    (:then
      (bind _returnvalue_3 (Game|Damage|ApplyPointDamage _asbp_enemy (Variables|Default|GetDamageValue) HitLocation HitInfo))
      ;[1 0 0] 向AI报告伤害感知事件
      (Utilities|IsValid _vrcharacter
        (:Is%20Valid
          (Class|AISenseDamage|ReportDamageEvent _asbp_enemy _vrcharacter _returnvalue_3 (Class|VRBaseCharacter|GetVRLocation _vrcharacter) "0, 0, 0" "None"))
        (:Is%20Not%20Valid
          _)))
    (:CastFailed
      (if (Physics|IsSimulatingPhysics Hit%20Comp "None")
        (Physics|AddImpulseatLocation (Variables|Default|GetHit%20Comp) (/ (Transformation|GetVelocity) 1e+01) (Transformation|GetActorLocation) "None"))
      ;[1 1 1] 弹坑效果
      (bind _returnvalue_4 (Rendering|Decal|SpawnDecalatLocation (CallFunction|GetRandomHoleDecals (Variables|Default|GetDecal%20Material)) "8.000000,8.000000,8.000000" HitLocation _returnvalue_2 1e+01))
      (Utilities|IsValid _returnvalue_4
        (:Is%20Valid
          (Transformation|AttachComponentToComponent _returnvalue_4 (Variables|Default|GetHit%20Comp) "None" "KeepWorld" "KeepWorld" "KeepRelative" true))
        (:Is%20Not%20Valid
          _))
      (Niagara|SpawnSystematLocation "/Game/MyVRProject/Assets/NigaraSystem/NS_BulletImpact.NS_BulletImpact" HitLocation _returnvalue_2 "0.500000,0.500000,0.500000")))
  (Actor|DestroyActor))

(event Custom|BulletHit_Server
  (params (HitActor :type Object%20Object%20Reference) (Hit%20Comp :type Primitive%20Component%20Object%20Reference) (HitLocation :type Vector%20%28by%20ref%29) (HitNormal :type Vector) (HitInfo :type Hit%20Result%20Structure%20%28by%20ref%29))
  (CallFunction|BulletHitMulti HitActor Hit%20Comp HitLocation HitNormal HitInfo))

(event Custom|BulletHit_Multi
  (params (HitActor :type Object%20Object%20Reference) (Hit%20Comp :type Primitive%20Component%20Object%20Reference) (HitLocation :type Vector%20%28by%20ref%29) (HitNormal :type Vector) (HitInfo :type Hit%20Result%20Structure%20%28by%20ref%29))
  (CallFunction|BulletHit HitActor Hit%20Comp HitLocation HitNormal HitInfo))

(event Collision|EventHit
  (params (MyComp :type Primitive%20Component%20Object%20Reference) (Other :type Actor%20Object%20Reference) (OtherComp :type Primitive%20Component%20Object%20Reference) (bSelfMoved :type Boolean) (HitLocation :type Vector :default "0, 0, 0") (HitNormal :type Vector :default "0, 0, 0") (NormalImpulse :type Vector :default "0, 0, 0") (Hit :type Hit%20Result%20Structure%20%28by%20ref%29))
  (CallFunction|BulletHitServer Other OtherComp HitLocation HitNormal Hit))

(fn ConstructionScript)

(fn GetRandomHoleDecals
  (params (Decal%20Material :type Array%20of%20Material%20Interface%20Object%20References))
  (return (Utilities|Array|Get(acopy) Decal%20Material (Math|Random|RandomIntegerinRange 0 (- (Utilities|Array|Length Decal%20Material) 1)))))