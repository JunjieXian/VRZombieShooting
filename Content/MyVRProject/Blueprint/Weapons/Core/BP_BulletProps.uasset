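; VR ammo pickup that adds bullets to a player's reserve when gripped.
; On grip, it resolves the BP_MyVRCharacter behind the gripping controller and passes it along a Server-to-Multi event chain, named for network replication.
; The final event adds BulletsNum to the character's TotalBullets, plays the pickup sound, refreshes the bullet count widget and destroys the actor.
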(event Custom|GetBulletsProps_Server
  (params (VRCharacter :type BP%20My%20VR%20Character%20Object%20Reference))
  (CallFunction|GetBulletsPropsMulti VRCharacter))

(event Custom|GetBulletsProps_Multi
  (params (VRCharacter :type BP%20My%20VR%20Character%20Object%20Reference))
  (CallFunction|GetBulletsProps VRCharacter))

(event Custom|GetBulletsProps
  (params (VRCharacter :type BP%20My%20VR%20Character%20Object%20Reference))
  (Variables|/Game/MyVRProject/Blueprint/Charactor/BP_MyVRCharacter.BP_MyVRCharacter_C|SetTotalBullets VRCharacter (+ (Variables|/Game/MyVRProject/Blueprint/Charactor/BP_MyVRCharacter.BP_MyVRCharacter_C|GetTotalBullets VRCharacter) (Variables|Default|GetBulletsNum)))
  (Audio|PlaySoundatLocation "/Game/MyVRProject/Assets/Sounds/Gun/弹药拾取.弹药拾取" (Transformation|GetActorLocation) "0, 0, 0" 1.0 1.0 0.0 0 0 0 0)
  (Default|UpdateBulletNumWidget VRCharacter)
  (Actor|DestroyActor))

(event EventBeginPlay)

(event Collision|EventActorBeginOverlap
  (params (OtherActor :type Actor%20Object%20Reference)))

(event EventTick
  (params (DeltaSeconds :type Float%20%28single-precision%29)))

(event EventOnGrip
  (params (GrippingController :type Grip%20Motion%20Controller%20Component%20Object%20Reference) (GripInformation :type BP%20Actor%20Grip%20Information%20Structure%20%28by%20ref%29))
  (bind _asbp_my_vrcharacter (Utilities|Casting|CastToBP_MyVRCharacter (Pawn|GetControlledPawn (Game|GetInstigatorController (Components|GetOwner GrippingController)))))
  (CallFunction|GetBulletsPropsServer _asbp_my_vrcharacter))

(fn ConstructionScript)