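; VR AR4 automatic rifle that grips, loads, chambers and fires, updating the holder's bullet-count widget.
; A held magazine snaps in on overlapping AmmoAttachment, and pulling the charging slider enables firing.
; Trigger use routes through server-to-multicast events into a looping timer that spends ammo and spawns bullets, muzzle flash, sound and ejected shells.
; Each shot adds GS_GunTools recoil, dampened by a secondary grip, until release or empty.
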(event OnComponentBeginOverlap(AmmoAttachment)
  (params (OverlappedComponent :type Primitive%20Component%20Object%20Reference) (OtherActor :type Actor%20Object%20Reference) (OtherComp :type Primitive%20Component%20Object%20Reference) (OtherBodyIndex :type Integer) (bFromSweep :type Boolean) (SweepResult :type Hit%20Result%20Structure%20%28by%20ref%29))
  ;[1 0.2684 0] 弹夹处理
  (bind _bisheld (Class|VRGripInterface|IsHeld))
  (if _bisheld
    (Utilities|IsValid (Variables|Default|GetAmmo)
      (:Is%20Not%20Valid
        (bind _asbp_ar4_ammo (Utilities|Casting|CastToBP_AR4_Ammo OtherActor))
        (if (Variables|/Game/MyVRProject/Blueprint/Weapons/AR4/BP_AR4_Ammo.BP_AR4_Ammo_C|GetisGrip _asbp_ar4_ammo) ; 临时解决取下弹夹isHeld调用为false的问题
          (bind _output_get (Variables|Default|SetAmmo _asbp_ar4_ammo))
          (Default|SetonLoadServer _output_get self "AmmoSlot" true)
          (bind _vrcharacter (Variables|Default|GetVRCharacter)
            (:then
              (Default|UpdateBulletNumWidget _vrcharacter (Variables|/Game/MyVRProject/Blueprint/Weapons/Core/BP_Ammo.BP_Ammo_C|GetCurrentBullets (Variables|Default|GetAmmo))))
            (:else)))))))

(event OnComponentEndOverlap(AmmoAttachment)
  (params (OverlappedComponent :type Primitive%20Component%20Object%20Reference) (OtherActor :type Actor%20Object%20Reference) (OtherComp :type Primitive%20Component%20Object%20Reference) (OtherBodyIndex :type Integer))
  ;[1 0.2684 0] 弹夹处理
  (if (== OtherActor (Variables|Default|GetAmmo))
    (Default|SetonLoadServer (Variables|Default|GetAmmo) 0 "AmmoSlot" false)
    (Variables|Default|SetAmmo 0)
    (Variables|Default|SetCanFire false)
    (bind _vrcharacter (Variables|Default|GetVRCharacter)
      (:then
        (Default|UpdateBulletNumWidget _vrcharacter))
      (:else))))

(event OnSliderHitPoint(LoadSlider)
  (params (SliderProgressPoint :type Float%20%28single-precision%29))
  ;[1 0 0.04575] 子弹上膛逻辑
  (if (<= SliderProgressPoint 0.9)
    (Audio|PlaySoundatLocation "/Game/MyVRProject/Assets/Sounds/Gun/拉栓01.拉栓01" (Transformation|GetWorldLocation (Variables|Default|GetLoadSlider)) "0, 0, 0" 1.0 1.0 0.0 0 0 0 0)))

(event OnSliderFinishedLerping(LoadSlider)
  (params (FinalProgress :type Float%20%28single-precision%29))
  ;[1 0 0.04575] 子弹上膛逻辑
  (Variables|Default|SetFinal%20Progress FinalProgress)
  (bind _alpha (Timeline|LoadSlideTimeline Play)
    (:Update
      (Class|VRSliderComponent|SetSliderProgress (Variables|Default|GetLoadSlider) (Math|Float|Lerp (Variables|Default|GetFinal%20Progress) 1.0 _alpha)))
    (:Finished
      (Utilities|CheckonLoad
        (:Can
          (Variables|Default|SetCanFire true))))))

(event Custom|Fire
  (bind _shootarrow (Variables|Default|GetShootArrow))
  (bind _shellemptyarrow (Variables|Default|GetShellEmptyArrow))
  (bind _guntoolsreference (Variables|Default|GetGunToolsReference))
  (bind _ammo (Variables|Default|GetAmmo))
  (bind _returnvalue (Transformation|GetWorldTransform _shootarrow))
  ;[0 1 0.4994] Fire Logic
  (Utilities|IsValid _ammo
    (:Is%20Valid
      (if (> (Variables|/Game/MyVRProject/Blueprint/Weapons/Core/BP_Ammo.BP_Ammo_C|GetCurrentBullets _ammo) 0)
        (bind _output_get (Variables|/Game/MyVRProject/Blueprint/Weapons/Core/BP_Ammo.BP_Ammo_C|SetCurrentBullets _ammo (- (Variables|/Game/MyVRProject/Blueprint/Weapons/Core/BP_Ammo.BP_Ammo_C|GetCurrentBullets _ammo) 1)))
        (bind _vrcharacter (Variables|Default|GetVRCharacter)
          (:then
            (Default|UpdateBulletNumWidget _vrcharacter _output_get)
            (Game|SpawnActorfromClass "/Game/MyVRProject/Blueprint/Weapons/Core/BP_Bullet.BP_Bullet_C" (Math|Transform|MakeTransform (.location _returnvalue) (Math|Rotator|MakeRotfromZ (Math|Vector|GetForwardVector _shootarrow)) (.scale _returnvalue)) "Undefined" 0 (Variables|Default|GetDamage) (Variables|Default|GetVRCharacter) 0)
            (Niagara|SpawnSystematLocation "/Game/MyVRProject/Assets/NigaraSystem/NS_AR_Muzzleflash_ONCE.NS_AR_Muzzleflash_ONCE" (Transformation|GetSocketLocation (Variables|Default|GetSkeletalMeshComponent) "b_gun_muzzleflash") (Transformation|GetWorldRotation (Variables|Default|GetShootArrow)) "0.500000,0.500000,0.500000")
            (Audio|PlaySoundatLocation "/Game/MyVRProject/Assets/Sounds/Gun/M4A1-1枪声.M4A1-1枪声" (Transformation|GetWorldLocation (Variables|Default|GetShootArrow)) "0, 0, 0" 1.0 1.0 0.0 0 0 0 0) ; 开枪音效
            ;;[1 1 1] 空弹壳处理
            (bind _returnvalue_2 (Game|SpawnActorfromClass "/Game/MyVRProject/Blueprint/Weapons/Core/BP_ShellEmpty.BP_ShellEmpty_C" (Transformation|GetWorldTransform _shellemptyarrow) "Undefined" 0 0))
            (Physics|AddImpulse (Variables|/Game/MyVRProject/Blueprint/Weapons/Core/BP_ShellEmpty.BP_ShellEmpty_C|GetShell _returnvalue_2) (* (Math|Vector|GetForwardVector _shellemptyarrow) 4.0) "None" false)
            ;;[1 1 1] GS Gun Tools实现后坐力
            (Class|GSGunTools|AddRecoilInstance _guntoolsreference (CallFunction|CalculateGunRecoil (Variables|Default|GetisSecondaryGriped) _guntoolsreference 24.0) "0, 0, 0"))
          (:else
            (Class|VRGripInterface|OnEndUsed :!label _label)
            (Audio|PlaySoundatLocation "/Game/MyVRProject/Assets/Sounds/Gun/空枪无法触发扳机.空枪无法触发扳机" "0, 0, 0" "0, 0, 0" 1.0 1.0 0.0 0 0 0 0) ; 空弹夹时扳机音效
            (Variables|Default|SetCanFire false)))
        (else
          (goto _label))))
    (:Is%20Not%20Valid
      (goto _label))))

(event Custom|GunFire
  ;[0 1 0.4994] Fire Logic
  (CallFunction|Fire)
  (bind _returnvalue (Utilities|Time|SetTimerbyEvent (delegate Custom|Fire) (Variables|Default|GetShootSpeed) true))
  (Variables|Default|SetShootTimer _returnvalue))

(event Custom|GunFire_Multi
  ;[0 1 0.4994] Fire Logic
  (CallFunction|GunFire))

(event Custom|EndGunFire
  ;[0 1 0.4994] Fire Logic
  ;;[0.1698 1 0.7575] EndFire
  (Utilities|Time|ClearandInvalidateTimerbyHandle (Variables|Default|GetShootTimer)))

(event Custom|EndGunFire_Server
  ;[0 1 0.4994] Fire Logic
  ;;[0.1698 1 0.7575] EndFire
  (CallFunction|EndGunFireMulti))

(event Custom|EndGunFire_Multi
  ;[0 1 0.4994] Fire Logic
  ;;[0.1698 1 0.7575] EndFire
  (CallFunction|EndGunFire))

(event Custom|GunFire_Server
  ;[0 1 0.4994] Fire Logic
  (CallFunction|GunFireMulti))

(event EventBeginPlay
  (|CallParentFunction)
  (bind _returnvalue (Class|VRGripScriptBase|GetGripScriptbyClass "/Script/VRExpansionPlugin.GS_GunTools")
    (:OnSucceeded
      (bind _asgs_gun_tools (Utilities|Casting|CastToGS_GunTools _returnvalue))
      (Variables|Default|SetGunToolsReference _asgs_gun_tools))))

(event Collision|EventActorBeginOverlap
  (params (OtherActor :type Actor%20Object%20Reference))
  (|CallParentFunction OtherActor) ; 此节点被禁用，将不会被调用。\n从引脚连出引线来编译功能。
)

(event EventTick
  (params (DeltaSeconds :type Float%20%28single-precision%29))
  (|CallParentFunction DeltaSeconds) ; 此节点被禁用，将不会被调用。\n从引脚连出引线来编译功能。
)

(event EventOnUsed
  ;[0 1 0.4994] Fire Logic
  (if (Variables|Default|GetCanFire) ; 是否已上膛
    (CallFunction|GunFireServer)
    (else
      (Audio|PlaySoundatLocation "/Game/MyVRProject/Assets/Sounds/Gun/空枪无法触发扳机.空枪无法触发扳机" "0, 0, 0" "0, 0, 0" 1.0 1.0 0.0 0 0 0 0) ; 空弹夹.未上膛时扳机音效
      (Variables|Default|SetCanFire false))))

(event EventOnGrip
  (params (GrippingController :type Grip%20Motion%20Controller%20Component%20Object%20Reference) (GripInformation :type BP%20Actor%20Grip%20Information%20Structure%20%28by%20ref%29))
  (bind _asbp_my_vrcharacter (Utilities|Casting|CastToBP_MyVRCharacter (Components|GetOwner GrippingController)))
  (bind _output_get (Variables|Default|SetVRCharacter _asbp_my_vrcharacter))
  (bind _ammo (Variables|Default|GetAmmo)
    (:then
      (Default|UpdateBulletNumWidget _output_get (Variables|/Game/MyVRProject/Blueprint/Weapons/Core/BP_Ammo.BP_Ammo_C|GetCurrentBullets _ammo)))
    (:else)))

(event EventOnEndUsed
  ;[0 1 0.4994] Fire Logic
  ;;[0.1698 1 0.7575] EndFire
  (CallFunction|EndGunFireServer))

(event EventOnSecondaryGrip
  (params (GripOwningController :type Grip%20Motion%20Controller%20Component%20Object%20Reference) (SecondaryGripComponent :type Scene%20Component%20Object%20Reference) (GripInformation :type BP%20Actor%20Grip%20Information%20Structure%20%28by%20ref%29))
  ;[0 1 0.4994] Fire Logic
  ;;[1 1 1] GS Gun Tools实现后坐力
  (Variables|Default|SetisSecondaryGriped true))

(event EventOnSecondaryGripRelease
  (params (GripOwningController :type Grip%20Motion%20Controller%20Component%20Object%20Reference) (ReleasingSecondaryGripComponent :type Scene%20Component%20Object%20Reference) (GripInformation :type BP%20Actor%20Grip%20Information%20Structure%20%28by%20ref%29))
  ;[0 1 0.4994] Fire Logic
  ;;[1 1 1] GS Gun Tools实现后坐力
  (Variables|Default|SetisSecondaryGriped false))

(event EventOnGripRelease
  (params (ReleasingController :type Grip%20Motion%20Controller%20Component%20Object%20Reference) (GripInformation :type BP%20Actor%20Grip%20Information%20Structure%20%28by%20ref%29) (bWasSocketed :type Boolean))
  (Default|UpdateBulletNumWidget (Variables|Default|GetVRCharacter))
  (Variables|Default|SetVRCharacter 0))

(fn ConstructionScript
  (|CallParentFunction))

(fn CalculateGunRecoil
  (params (HasSecondaryGrip :type Boolean) (GSGunTools :type GS%20Gun%20Tools%20Object%20Reference) (DivideValue :type Float%20%28double-precision%29))
  (bind _maxrecoiltranslation (Variables|/Script/VRExpansionPlugin.GS_GunTools|GetMaxRecoilTranslation GSGunTools))
  (bind _maxrecoilrotation (Variables|/Script/VRExpansionPlugin.GS_GunTools|GetMaxRecoilRotation GSGunTools))
  (bind _maxrecoilrotation_2 (Variables|/Script/VRExpansionPlugin.GS_GunTools|GetMaxRecoilRotation GSGunTools))
  (if HasSecondaryGrip
    (return (Math|Transform|MakeTransform (/ (Math|Vector|MakeVector (.x _maxrecoiltranslation) (.y _maxrecoiltranslation) (.z _maxrecoiltranslation)) DivideValue) (Math|Rotator|MakeRotator (/ (.x _maxrecoilrotation) DivideValue) (.y _maxrecoilrotation) (.z _maxrecoilrotation))))
    (else
      (return (Math|Transform|MakeTransform (Variables|/Script/VRExpansionPlugin.GS_GunTools|GetMaxRecoilTranslation GSGunTools) (Math|Rotator|MakeRotator (.x _maxrecoilrotation_2) (.y _maxrecoilrotation_2) (.z _maxrecoilrotation_2)))))))