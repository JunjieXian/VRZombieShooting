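; AR4 magazine actor for VR weapons that can be gripped, loaded into a weapon socket and removed.
; SetOnLoad either snaps it to the parent's socket with physics off or detaches it, keeping single-hand gripping allowed and playing the matching sound.
; Server and Multi events relay the load state for multiplayer.
; Grip events track IsGrip as a temporary workaround for an isHeld bug that breaks reloading a removed magazine.
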(event Custom|SetOnLoad
  (params (ParentActor :type Actor%20Object%20Reference) (SocketName :type Name) (load :type Boolean))
  ;[1 1 1] 弹夹装载事件
  (if load
    (Transformation|AttachActorToActor ParentActor SocketName "SnapToTarget" "SnapToTarget" "KeepRelative" true)
    (Physics|SetSimulatePhysics (Variables|Default|GetStaticMeshComponent) false)
    (Variables|Default|SetVRGripInterfaceSettings (Utilities|Struct|MakeBPInterfaceProperties false false "DropOnTeleport" false "InteractiveHybridCollisionWithPhysics" "InteractiveHybridCollisionWithPhysics" "SG_None" "ClientSide_Authoritive" "NotWhenCollidingOrDoubleGripping")) ; SimulateOnDrop关闭
    (Audio|PlaySoundatLocation "/Game/MyVRProject/Assets/Sounds/Gun/弹夹装载.弹夹装载" (Transformation|GetActorLocation) "0, 0, 0" 1.0 1.0 0.0 0 0 0 0)
    (else
      (Variables|Default|SetVRGripInterfaceSettings (Utilities|Struct|MakeBPInterfaceProperties false false "DropOnTeleport" true "InteractiveHybridCollisionWithPhysics" "InteractiveHybridCollisionWithPhysics" "SG_None" "ClientSide_Authoritive" "NotWhenCollidingOrDoubleGripping"))
      (Transformation|DetachFromActor "KeepRelative" "KeepRelative" "KeepRelative")
      (Audio|PlaySoundatLocation "/Game/MyVRProject/Assets/Sounds/Gun/弹夹取出.弹夹取出" (Transformation|GetActorLocation) "0, 0, 0" 1.0 1.0 0.0 0 0 0 0))))

(event Custom|SetOnLoad_Server
  (params (ParentActor :type Actor%20Object%20Reference) (SocketName :type Name) (load :type Boolean))
  ;[1 1 1] 弹夹装载事件
  (CallFunction|SetonLoadMulti ParentActor SocketName load))

(event Custom|SetOnLoad_Multi
  (params (ParentActor :type Actor%20Object%20Reference) (SocketName :type Name) (load :type Boolean))
  ;[1 1 1] 弹夹装载事件
  (CallFunction|SetonLoad ParentActor SocketName load))

(event EventBeginPlay)

(event EventOnGrip
  (params (GrippingController :type Grip%20Motion%20Controller%20Component%20Object%20Reference) (GripInformation :type BP%20Actor%20Grip%20Information%20Structure%20%28by%20ref%29))
  ;[1 0 0.08944] 临时解决取下弹夹时，调用isHeld为false导致二次上弹夹失败。
  ; 未知BUG，，后期验证解决。
  (Variables|Default|SetisGrip true))

(event EventOnGripRelease
  (params (ReleasingController :type Grip%20Motion%20Controller%20Component%20Object%20Reference) (GripInformation :type BP%20Actor%20Grip%20Information%20Structure%20%28by%20ref%29) (bWasSocketed :type Boolean))
  ;[1 0 0.08944] 临时解决取下弹夹时，调用isHeld为false导致二次上弹夹失败。
  ; 未知BUG，，后期验证解决。
  (Variables|Default|SetisGrip false))

(fn ConstructionScript
  (|CallParentFunction))