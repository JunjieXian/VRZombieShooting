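; BP_MainMenuPawn is the VR pawn for the main menu, letting the player click UI widgets with either hand.
; On BeginPlay it adds the VREInputMappingContext to the local player's Enhanced Input subsystem.
; The left and right UseHeldObject actions press and release a simulated left mouse button on that hand's widget interaction component.
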(event Input|EnhancedActionEvents|EnhancedInputActionUseHeldObjectLeft
  (params (ActionValue :type Boolean) (ElapsedSeconds :type Float%20%28double-precision%29) (TriggeredSeconds :type Float%20%28double-precision%29) (InputAction :type Input%20Action%20Object%20Reference :default "/Game/VRE/Input/Actions/UseHeldObjectLeft.UseHeldObjectLeft"))
  (bind _lwidgetinteraction (Variables|Default|GetLWidgetInteraction))
  (:Started
    (Class|WidgetInteractionComponent|PressPointerKey _lwidgetinteraction "LeftMouseButton"))
  (:Completed
    (Class|WidgetInteractionComponent|ReleasePointerKey _lwidgetinteraction "LeftMouseButton")))

(event Input|EnhancedActionEvents|EnhancedInputActionUseHeldObjectRight
  (params (ActionValue :type Boolean) (ElapsedSeconds :type Float%20%28double-precision%29) (TriggeredSeconds :type Float%20%28double-precision%29) (InputAction :type Input%20Action%20Object%20Reference :default "/Game/VRE/Input/Actions/UseHeldObjectRight.UseHeldObjectRight"))
  (bind _rwidgetinteraction (Variables|Default|GetRWidgetInteraction))
  (:Started
    (Class|WidgetInteractionComponent|PressPointerKey _rwidgetinteraction "LeftMouseButton"))
  (:Completed
    (Class|WidgetInteractionComponent|ReleasePointerKey _rwidgetinteraction "LeftMouseButton")))

(event EventBeginPlay
  (bind _returnvalue (Game|GetPlayerController 0))
  (bind _returnvalue_2 (PlayerController|LocalPlayerSubsystems|GetEnhancedInputLocalPlayerSubsystem _returnvalue))
  (Utilities|IsValid _returnvalue_2
    (:Is%20Valid
      (Input|AddMappingContext _returnvalue_2 "/Game/VRE/Input/VREInputMappingContext.VREInputMappingContext" 0 "(bIgnoreAllPressedKeysUntilRelease=True,bForceImmediately=False)"))))

(event Collision|EventActorBeginOverlap
  (params (OtherActor :type Actor%20Object%20Reference)))

(event EventTick
  (params (DeltaSeconds :type Float%20%28single-precision%29)))

(fn ConstructionScript)